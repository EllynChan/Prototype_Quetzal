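; BP_Core is a damageable enemy core actor with a world-space health bar, destroyed when its health runs out.
; Each tick it turns the HealthBar widget toward the player camera and writes the current health fraction into WBP_Core.
; AnyDamage subtracts clamped health and, at zero, sets IsDead and calls OnDeath, which destroys the actor.
; A BP_Portal spawn at the actor's transform is present but disconnected, so it never runs.
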(event Custom|Event%20OnDeath
  (Actor|DestroyActor))

(event Game|Damage|EventAnyDamage
  (params (Damage :type Float%20%28single-precision%29) (DamageType :type Damage%20Type%20Object%20Reference) (InstigatedBy :type Controller%20Object%20Reference) (DamageCauser :type Actor%20Object%20Reference))
  (if (not (Variables|Default|GetIsDead))
    (Variables|Default|SetCurrHealth (Math|Float|Clamp(Float) (- (Variables|Default|GetCurrHealth) Damage) 0.0 (Variables|Default|GetMaxHealth)))
    (if (== (Math|Float|Clamp(Float) (- (Variables|Default|GetCurrHealth) Damage) 0.0 (Variables|Default|GetMaxHealth)) 0.0)
      (Variables|Default|SetIsDead true)
      (CallFunction|EventonDeath))))

(event EventTick
  (params (DeltaSeconds :type Float%20%28single-precision%29))
  (bind _health_bar (Variables|Default|GetHealth%20Bar))
  (Transformation|SetWorldRotation _health_bar (Math|Rotator|FindRelativeLookatRotation (Math|Conversions|ToTransform(Vector) (Transformation|GetWorldLocation _health_bar)) (Transformation|GetWorldLocation (Variables|/Script/Engine.PlayerCameraManager|GetTransformComponent (Game|GetPlayerCameraManager 0)))) false false)
  (bind _aswbp_core (Utilities|Casting|CastToWBP_Core (UserInterface|GetWidget (Variables|Default|GetHealth%20Bar))))
  (Progress|SetPercent (Variables|/Game/Dynamic/BluePrints/UI/WBP_Core.WBP_Core_C|GetEnemy_HealthBar _aswbp_core) (/ (Variables|Default|GetCurrHealth) (Variables|Default|GetMaxHealth))))

(fn ConstructionScript)