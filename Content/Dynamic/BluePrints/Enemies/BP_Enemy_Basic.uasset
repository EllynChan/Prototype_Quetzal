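; Basic enemy that periodically shoots at the player and drops a collectible when killed.
; A looping timer set on BeginPlay spawns BP_Enemy_Bullet aimed at the player character.
; Tick turns the widget health bar toward the camera and updates its fill.
; AnyDamage lowers clamped health, but its death check subtracts damage again, so death can trigger early, spawning BP_Collectible and destroying the enemy.
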(event Custom|Fire%20Projectile
  (bind _returnvalue (Transformation|GetActorLocation))
  (Game|SpawnActorfromClass "/Game/Dynamic/BluePrints/Projectiles/BP_Enemy_Bullet.BP_Enemy_Bullet_C" (Math|Transform|MakeTransform _returnvalue (Math|Rotator|FindLookatRotation _returnvalue (Transformation|GetActorLocation (Game|GetPlayerCharacter 0)))) "AdjustIfPossibleButAlwaysSpawn" "MultiplyWithRoot" self 0))

(event Custom|Event%20OnDeath
  (bind _defaultsceneroot (Variables|Default|GetDefaultSceneRoot))
  (bind _returnvalue (Transformation|GetWorldTransform _defaultsceneroot))
  (bind _returnvalue_2 (Game|SpawnActorfromClass "/Game/Dynamic/BluePrints/Interactables/BP_Collectible.BP_Collectible_C" (Math|Transform|MakeTransform (.location _returnvalue) (.rotation _returnvalue) "1.000000,1.000000,1.000000") "AlwaysSpawn" "MultiplyWithRoot" 0 0))
  (Actor|DestroyActor))

(event Game|Damage|EventAnyDamage
  (params (Damage :type Float%20%28single-precision%29) (DamageType :type Damage%20Type%20Object%20Reference) (InstigatedBy :type Controller%20Object%20Reference) (DamageCauser :type Actor%20Object%20Reference))
  (if (not (Variables|Default|GetIsDead))
    (Variables|Default|SetCurrHealth (Math|Float|Clamp(Float) (- (Variables|Default|GetCurrHealth) Damage) 0.0 (Variables|Default|GetMaxHealth)))
    (if (== (Math|Float|Clamp(Float) (- (Variables|Default|GetCurrHealth) Damage) 0.0 (Variables|Default|GetMaxHealth)) 0.0)
      (Variables|Default|SetIsDead true)
      (CallFunction|EventonDeath))))

(event EventTick
  (params (DeltaSeconds :type Float%20%28single-precision%29))
  (bind _health_bar (Variables|Default|GetHealth%20Bar))
  (Transformation|SetWorldRotation _health_bar (Math|Rotator|FindRelativeLookatRotation (Math|Conversions|ToTransform(Vector) (Transformation|GetWorldLocation _health_bar)) (Transformation|GetWorldLocation (Variables|/Script/Engine.PlayerCameraManager|GetTransformComponent (Game|GetPlayerCameraManager 0)))) false false)
  (bind _aswbp_enemy_health_bar (Utilities|Casting|CastToWBP_Enemy_HealthBar (UserInterface|GetWidget (Variables|Default|GetHealth%20Bar))))
  (Progress|SetPercent (Variables|/Game/Dynamic/BluePrints/UI/WBP_Enemy_HealthBar.WBP_Enemy_HealthBar_C|GetEnemy_HealthBar _aswbp_enemy_health_bar) (/ (Variables|Default|GetCurrHealth) (Variables|Default|GetMaxHealth))))

(event EventBeginPlay
  (Utilities|Time|SetTimerbyEvent (delegate Custom|Fire%20Projectile) (Variables|Default|GetFiringRate) true))

(fn ConstructionScript)