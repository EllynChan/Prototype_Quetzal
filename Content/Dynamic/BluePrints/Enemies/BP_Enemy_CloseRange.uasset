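; Melee enemy that chases the player, attacks up close and drops a BP_Collectible on death.
; Tick turns its health bar widget toward the camera, updates it, and drives swept, direct movement toward the player without pathfinding.
; Within ChaseDistance it deals fixed damage, then pauses on a delay before acting again.
; Incoming damage lowers clamped health, but the death check subtracts damage again, so it can die with health remaining.
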(event Custom|ChasePlayer
  (bind _returnvalue (Game|GetPlayerCharacter 0))
  (bind _returnvalue_2 (Transformation|GetActorLocation))
  (bind _returnvalue_3 (Transformation|GetActorLocation _returnvalue))
  (if (< (Transformation|GetDistanceTo (Game|Player|GetPlayerPawn 0)) (Variables|Default|GetChaseDistance))
    (Variables|Default|SetCanAct false)
    (CallFunction|Attack)
    (else
      (Transformation|SetActorLocationAndRotation (+ (Transformation|GetWorldLocation (Variables|Default|GetSphere%20Collider)) (* (Math|Vector|Normalize (- _returnvalue_3 _returnvalue_2)) (Utilities|Time|GetWorldDeltaSeconds) (Variables|Default|GetChaseSpeed))) (Math|Rotator|FindLookatRotation _returnvalue_2 _returnvalue_3) true))))

(event Custom|Event%20OnDeath
  (bind _sphere_collider (Variables|Default|GetSphere%20Collider))
  (bind _returnvalue (Transformation|GetWorldTransform _sphere_collider))
  (bind _returnvalue_2 (Game|SpawnActorfromClass "/Game/Dynamic/BluePrints/Interactables/BP_Collectible.BP_Collectible_C" (Math|Transform|MakeTransform (.location _returnvalue) (.rotation _returnvalue) "1.000000,1.000000,1.000000") "AlwaysSpawn" "MultiplyWithRoot" 0 0))
  (Actor|DestroyActor))

(event Custom|Attack
  (Game|Damage|ApplyDamage (Game|Player|GetPlayerPawn 0) 1e+01 0 0))

(event Game|Damage|EventAnyDamage
  (params (Damage :type Float%20%28single-precision%29) (DamageType :type Damage%20Type%20Object%20Reference) (InstigatedBy :type Controller%20Object%20Reference) (DamageCauser :type Actor%20Object%20Reference))
  (if (not (Variables|Default|GetIsDead))
    (Variables|Default|SetCurrHealth (Math|Float|Clamp(Float) (- (Variables|Default|GetCurrHealth) Damage) 0.0 (Variables|Default|GetMaxHealth)))
    (if (== (Math|Float|Clamp(Float) (- (Variables|Default|GetCurrHealth) Damage) 0.0 (Variables|Default|GetMaxHealth)) 0.0)
      (Variables|Default|SetIsDead true)
      (CallFunction|EventonDeath))))

(event EventTick
  (params (DeltaSeconds :type Float%20%28single-precision%29))
  (bind _health_bar (Variables|Default|GetHealth%20Bar))
  (Transformation|SetWorldRotation _health_bar (Math|Rotator|FindRelativeLookatRotation (Math|Conversions|ToTransform(Vector) (Transformation|GetWorldLocation _health_bar)) (Transformation|GetWorldLocation (Variables|/Script/Engine.PlayerCameraManager|GetTransformComponent (Game|GetPlayerCameraManager 0)))) false false)
  (bind _aswbp_enemy_health_bar (Utilities|Casting|CastToWBP_Enemy_HealthBar (UserInterface|GetWidget (Variables|Default|GetHealth%20Bar))))
  (Progress|SetPercent (Variables|/Game/Dynamic/BluePrints/UI/WBP_Enemy_HealthBar.WBP_Enemy_HealthBar_C|GetEnemy_HealthBar _aswbp_enemy_health_bar) (/ (Variables|Default|GetCurrHealth) (Variables|Default|GetMaxHealth)))
  (if (Variables|Default|GetCanAct)
    (CallFunction|ChasePlayer)
    (else
      (Utilities|FlowControl|Delay 2.0)
      (Variables|Default|SetCanAct true))))

(fn ConstructionScript)