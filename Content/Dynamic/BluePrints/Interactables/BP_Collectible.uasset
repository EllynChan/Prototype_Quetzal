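; BP_Collectible is a pickup that shows an on-screen widget when the player collects it.
; An overlap of its Box component by an actor tagged Player adds WBP_Collectible to the viewport and hides the pickup, with a boolean blocking repeat triggers.
; Chained delays remove the widget, then destroy the actor.
; A lifespan set at BeginPlay also destroys the pickup after a fixed time.
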(event OnComponentBeginOverlap(Box)
  (params (OverlappedComponent :type Primitive%20Component%20Object%20Reference) (OtherActor :type Actor%20Object%20Reference) (OtherComp :type Primitive%20Component%20Object%20Reference) (OtherBodyIndex :type Integer) (bFromSweep :type Boolean) (SweepResult :type Hit%20Result%20Structure%20%28by%20ref%29))
  (if (Actor|ActorHasTag OtherActor "Player")
    (if (Variables|Default|GetShouldAddWidget)
      (bind _returnvalue (UserInterface|CreateWidget "/Game/Dynamic/BluePrints/UI/WBP_Collectible.WBP_Collectible_C"))
      (UserInterface|Viewport|AddtoViewport _returnvalue 0)
      (Variables|Default|SetShouldAddWidget false)
      (Rendering|SetActorHiddenInGame true)
      (Utilities|FlowControl|Delay 2.0)
      (Widget|RemovefromParent _returnvalue)
      (Utilities|FlowControl|Delay 2.0)
      (Actor|DestroyActor))))

(event Collision|EventActorBeginOverlap
  (params (OtherActor :type Actor%20Object%20Reference)))

(event EventTick
  (params (DeltaSeconds :type Float%20%28single-precision%29)))

(event EventBeginPlay
  (Actor|SetLifeSpan 2e+02))

(fn ConstructionScript)