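; BP_CollectibleKey is a collectible key that unlocks a level portal when the player picks it up.
; A box overlap from a Player-tagged actor fires once, guarded by a flag, showing a pickup widget and hiding the key.
; It points the referenced PortalActor at the hardcoded WhiteBox2 level, then reveals it and enables its query collision.
; After short delays it removes the widget, then destroys itself.
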(event OnComponentBeginOverlap(Box)
  (params (OverlappedComponent :type Primitive%20Component%20Object%20Reference) (OtherActor :type Actor%20Object%20Reference) (OtherComp :type Primitive%20Component%20Object%20Reference) (OtherBodyIndex :type Integer) (bFromSweep :type Boolean) (SweepResult :type Hit%20Result%20Structure%20%28by%20ref%29))
  (bind _portalactor (Variables|Default|GetPortalActor))
  (if (Actor|ActorHasTag OtherActor "Player")
    (if (Variables|Default|GetShouldAddWidget)
      (bind _returnvalue (UserInterface|CreateWidget "/Game/Dynamic/BluePrints/UI/WBP_CollectibleKey.WBP_CollectibleKey_C"))
      (UserInterface|Viewport|AddtoViewport _returnvalue 0)
      (Variables|Default|SetShouldAddWidget false)
      (Rendering|SetActorHiddenInGame true)
      (Variables|/Game/Static/StylizedPortalShaders/Blueprints/BP_Portal_Hole.BP_Portal_Hole_C|SetOpenLevelName _portalactor "WhiteBox2")
      (Rendering|SetActorHiddenInGame _portalactor false)
      (Collision|SetCollisionEnabled (Variables|/Game/Static/StylizedPortalShaders/Blueprints/BP_Portal_Hole.BP_Portal_Hole_C|GetCollision _portalactor) "QueryOnly")
      (Utilities|FlowControl|Delay 2.0)
      (Widget|RemovefromParent _returnvalue)
      (Utilities|FlowControl|Delay 1.0)
      (Actor|DestroyActor))))

(fn ConstructionScript)