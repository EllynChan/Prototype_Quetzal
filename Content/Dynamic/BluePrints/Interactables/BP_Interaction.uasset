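; BP_Interaction is an interactable that reveals a portal when the player presses E near it.
; Box overlap begin and end toggle a widget's visibility and a CanInteract flag, without filtering the overlapping actor.
; Tick polls the first player controller for E while the flag is set, then unhides PortalActor, enables query-only collision on it and destroys itself.
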(event OnComponentBeginOverlap(Box)
  (params (OverlappedComponent :type Primitive%20Component%20Object%20Reference) (OtherActor :type Actor%20Object%20Reference) (OtherComp :type Primitive%20Component%20Object%20Reference) (OtherBodyIndex :type Integer) (bFromSweep :type Boolean) (SweepResult :type Hit%20Result%20Structure%20%28by%20ref%29))
  (Rendering|SetVisibility (Variables|Default|GetWidget) true false)
  (Variables|Default|SetCanInteract true))

(event OnComponentEndOverlap(Box)
  (params (OverlappedComponent :type Primitive%20Component%20Object%20Reference) (OtherActor :type Actor%20Object%20Reference) (OtherComp :type Primitive%20Component%20Object%20Reference) (OtherBodyIndex :type Integer))
  (Rendering|SetVisibility (Variables|Default|GetWidget) false false)
  (Variables|Default|SetCanInteract false))

(event EventTick
  (params (DeltaSeconds :type Float%20%28single-precision%29))
  (bind _portalactor (Variables|Default|GetPortalActor))
  (if (and (Variables|Default|GetCanInteract) (Game|Player|IsInputKeyDown (Game|GetPlayerController 0) "E"))
    (Rendering|SetActorHiddenInGame _portalactor false)
    (Collision|SetCollisionEnabled (Variables|/Game/Static/StylizedPortalShaders/Blueprints/BP_Portal_Hole.BP_Portal_Hole_C|GetCollision _portalactor) "QueryOnly")
    (Actor|DestroyActor)))

(fn ConstructionScript)