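; BP_Instance_Damager_Cube is a hazard made of a 3D grid of scaled-up cube instances that kills the player character on overlap.
; The construction script fills DamageCubeInstances using nested loops, offsetting each instance by InstanceSpacing plus random jitter within InstanceRandomness, so the layout re-rolls whenever construction runs.
; Any overlap with that component casts the other actor to BP_ThirdPersonCharacter and calls EventOnDeath directly, with no damage amount.
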(event OnComponentBeginOverlap(DamageCubeInstances)
  (params (OverlappedComponent :type Primitive%20Component%20Object%20Reference) (OtherActor :type Actor%20Object%20Reference) (OtherComp :type Primitive%20Component%20Object%20Reference) (OtherBodyIndex :type Integer) (bFromSweep :type Boolean) (SweepResult :type Hit%20Result%20Structure%20%28by%20ref%29))
  (bind _asbp_third_person_character (Utilities|Casting|CastToBP_ThirdPersonCharacter OtherActor))
  (Default|EventonDeath _asbp_third_person_character))

(fn ConstructionScript
  (bind _instance_spacing (Variables|Default|GetInstance%20Spacing))
  (bind _instance_randomness (Variables|Default|GetInstance%20Randomness))
  (bind _returnvalue (* _instance_randomness -1.0))
  (bind _returnvalue_2 (Math|Random|RandomFloatinRange _returnvalue _instance_randomness))
  (for _index (range 0 10)
    (for _index_2 (range 0 3)
      (for _index_3 (range 0 10)
        (Components|InstancedStaticMesh|AddInstance (Variables|Default|GetDamageCubeInstances) (Math|Transform|MakeTransform (Math|Vector|MakeVector (+ (* _index _instance_spacing) _returnvalue_2) (+ (* _index_2 _instance_spacing) _returnvalue_2) (+ (* _index_3 _instance_spacing) _returnvalue_2)) "0, 0, 0" "3.000000,3.000000,3.000000") false)))))